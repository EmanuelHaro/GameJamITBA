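; Trigger actor that shows an in-game tutorial widget (TutorialPlacaIG) when BP_Personaje enters its box.
; On overlap it creates the widget if none is valid, shares the reference with the character, adds it to the viewport, shows the cursor, switches to UI-only input and pauses the game.
; The actor destroys itself when the character leaves the box, making the tutorial one-shot.
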(event OnComponentBeginOverlap(Box)
  (params (OverlappedComponent :type Primitive%20Component%20Object%20Reference) (OtherActor :type Actor%20Object%20Reference) (OtherComp :type Primitive%20Component%20Object%20Reference) (OtherBodyIndex :type Integer) (bFromSweep :type Boolean) (SweepResult :type Hit%20Result%20Structure%20%28by%20ref%29))
  (bind _returnvalue (Game|GetPlayerController 0))
  (bind _asbp_personaje (Utilities|Casting|CastToBP_Personaje OtherActor))
  (Utilities|IsValid (Variables|Default|GetWB%20IG%20Texto)
    (:Is%20Valid
      _)
    (:Is%20Not%20Valid
      (bind _returnvalue_2 (UserInterface|CreateWidget "/Game/UI/WB_TutorialPlacaIG.WB_TutorialPlacaIG_C"))
      (bind _output_get (Variables|Default|SetWB%20IG%20Texto _returnvalue_2))
      (Variables|/Game/BlueprintsMIOS/BP_Personaje.BP_Personaje_C|SetWB%20Texto%20IG _asbp_personaje _output_get)))
  (Variables|/Script/Engine.PlayerController|SetbShowMouseCursor _returnvalue true)
  (Input|SetInputModeUIOnly _returnvalue 0 "DoNotLock")
  (UserInterface|Viewport|AddtoViewport _returnvalue_2 0)
  (Game|SetGamePaused true))

(event OnComponentEndOverlap(Box)
  (params (OverlappedComponent :type Primitive%20Component%20Object%20Reference) (OtherActor :type Actor%20Object%20Reference) (OtherComp :type Primitive%20Component%20Object%20Reference) (OtherBodyIndex :type Integer))
  (Utilities|Casting|CastToBP_Personaje OtherActor)
  (Actor|DestroyActor))

(event EventBeginPlay)

(event Collision|EventActorBeginOverlap
  (params (OtherActor :type Actor%20Object%20Reference)))

(event EventTick
  (params (DeltaSeconds :type Float%20%28single-precision%29)))

(fn ConstructionScript)