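; Player character Blueprint with gravity inversion, physics object grabbing and a pause menu on L.
; Right mouse toggles inversion when allowed: a timeline rolls the actor, a Tick-fed gate applies vertical force, and look axes flip.
; Grab input traces from the camera for lighter physics bodies, carried by a PhysicsHandle targeting LocalizacionCaja until release.
; A looping timer traces along Z to set GravedadLineTrace, which is not read here.
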(event Custom|AgarrarObjetos
  (bind _cam (Variables|Default|Getcam))
  (bind _returnvalue (Transformation|GetWorldLocation _cam))
  ;[1 1 1] Agarrar Objeto
  (bind (_outhit _returnvalue_2) (Collision|LineTraceForObjects _returnvalue (+ _returnvalue (* (Math|Vector|GetForwardVector _cam) 7e+02)) (Utilities|Array|MakeArray "ObjectTypeQuery4") false 0 "None"))
  (if _returnvalue_2
    (if (< (Physics|GetMass (.HitComponent (Collision|BreakHitResult _outhit))) 1e+03)
      (Variables|Default|SetObejtoFisico (.HitComponent (Collision|BreakHitResult _outhit)))
      (Class|PhysicsHandleComponent|GrabComponentatLocation (Variables|Default|GetPhysicsHandle) (.HitComponent (Collision|BreakHitResult _outhit)) "None" (.Location (Collision|BreakHitResult _outhit)))
      (Variables|Default|SetagarroObjeto true)
      (Audio|PlaySound2D "/Game/Audios/swipe.swipe" 1.0 1.0 0.0 0 0)
      (Collision|SetCollisionResponsetoChannel (Variables|Default|GetObejtoFisico) "ECC_Pawn" "ECR_Ignore")
      (Class|PrimitiveComponent|SetAngularDamping (Variables|Default|GetObejtoFisico) 1e+01))))

(event Custom|SoltarObjeto
  (bind _obejtofisico (Variables|Default|GetObejtoFisico))
  ;[1 1 1] Soltar Objeto
  (if (Variables|Default|GetcambioGravedad)
    (Physics|SetEnableGravity (Variables|Default|GetObejtoFisico) true))
  (Physics|Components|PhysicsHandle|ReleaseComponent (Variables|Default|GetPhysicsHandle))
  (Variables|Default|SetagarroObjeto false)
  (Collision|SetCollisionResponsetoChannel _obejtofisico "ECC_Pawn" "ECR_Block")
  (Class|PrimitiveComponent|SetAllPhysicsLinearVelocity _obejtofisico "0, 0, 0" false)
  (Utilities|FlowControl|Delay 0.2)
  (Class|PrimitiveComponent|SetAngularDamping _obejtofisico 0.0))

(event EventBeginPlay
  (Utilities|Time|SetTimerbyFunctionName 0 "DetectarGravedad" 0.1 true))

(event EventTick
  (params (DeltaSeconds :type Float%20%28single-precision%29))
  ;[1 1 1] Invertir Gravedad
  (Utilities|FlowControl|Sequence
    (:then_0
      (Utilities|FlowControl|Gate true
        (:Exit
          (Physics|AddForce (Variables|Character|GetCharacterMovement) (Math|Vector|MakeVector 0.0 0.0 (* (Variables|Default|GetfuerzaGravedad) 1e+05))))))
    (:then_1
      (Physics|Components|PhysicsHandle|SetTargetLocation (Variables|Default|GetPhysicsHandle) (Transformation|GetWorldLocation (Variables|Default|GetLocalizacionCaja))))))

(event Input|ActionEvents|InputActionAgarrar
  (params (Key :type Key%20Structure :default "None"))
  (bind _agarroobjeto (Variables|Default|GetagarroObjeto))
  ;[1 1 1] Input Agarrar
  (:Pressed
    (if (not _agarroobjeto)
      (CallFunction|AgarrarObjetos)))
  (:Released
    (if _agarroobjeto
      (CallFunction|SoltarObjeto))))

(event Input|AxisEvents|InputAxisTurn
  (params (AxisValue :type Float%20%28single-precision%29))
  (Pawn|Input|AddControllerYawInput (Math|Float|SelectFloat (* AxisValue -1.0) AxisValue (Variables|Default|GetcambioGravedad))))

(event Input|AxisEvents|InputAxisLookUp
  (params (AxisValue :type Float%20%28single-precision%29))
  (Pawn|Input|AddControllerPitchInput (Math|Float|SelectFloat (* AxisValue -1.0) AxisValue (Variables|Default|GetcambioGravedad))))

(event Input|MouseEvents|RightMouseButton
  (params (Key :type Key%20Structure :default "None"))
  ;[1 1 1] Por si pinta cambiar la camar
)

(event Input|MouseEvents|RightMouseButton
  (params (Key :type Key%20Structure :default "None"))
  (bind _returnvalue (Transformation|GetActorRotation))
  ;[1 1 1] Invertir Gravedad
  (:Pressed
    (if (Variables|Default|GetpuedeInvertirGravedad)
      (Audio|PlaySound2D "/Game/Audios/swipe2.swipe2" 1.0 1.0 0.0 0 0)
      (Utilities|FlowControl|FlipFlop
        (:A
          (Variables|Default|SetcambioGravedad true)
          (Utilities|FlowControl|Sequence
            (:then_0
              (bind _ejex (Timeline|GirarPersonaje PlayFromStart)
                (:Update
                  (Transformation|SetActorRotation (Math|Rotator|MakeRotator _ejex (.pitch _returnvalue) (.yaw _returnvalue))))))
            (:then_1
              (Utilities|FlowControl|Gate true) ; enters at Open
            )))
        (:B
          (Variables|Default|SetcambioGravedad false)
          (Utilities|FlowControl|Sequence
            (:then_0
              (Timeline|GirarPersonaje Reverse))
            (:then_1
              (Utilities|FlowControl|Gate true) ; enters at Close
            )))))))

(event Input|KeyboardEvents|L
  (params (Key :type Key%20Structure :default "None"))
  (bind _returnvalue (Game|GetPlayerController 0))
  ;[1 1 1] Menu Pausa
  (:Pressed
    (Utilities|IsValid (Variables|Default|GetPause%20Menu%20Ref)
      (:Is%20Valid
        _)
      (:Is%20Not%20Valid
        (bind _returnvalue_2 (UserInterface|CreateWidget "/Game/UI/WB_Pausa.WB_Pausa_C"))
        (bind _output_get (Variables|Default|SetPause%20Menu%20Ref _returnvalue_2))))
    (Variables|/Script/Engine.PlayerController|SetbShowMouseCursor _returnvalue true)
    (Input|SetInputModeUIOnly _returnvalue _output_get "DoNotLock")
    (UserInterface|Viewport|AddtoViewport _output_get 0)
    (Game|SetGamePaused true)))

(fn ConstructionScript)

(fn DetectarGravedad
  (bind _returnvalue (Transformation|GetActorLocation))
  (bind (_x _y _z) (Math|Vector|BreakVector _returnvalue))
  (bind _returnvalue_2 (Collision|LineTraceForObjects _returnvalue (Math|Vector|MakeVector _x _y (* _z 1e+02)) (LocalVariables|GetWorldStatic) false 0 "None"))
  (if _returnvalue_2
    (Variables|Default|SetgravedadLineTrace true)
    (else
      (Variables|Default|SetgravedadLineTrace false))))