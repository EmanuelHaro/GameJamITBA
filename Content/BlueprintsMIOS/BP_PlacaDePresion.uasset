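; BP_PlacaDePresion is a pressure plate that switches a linked sliding wall (ParedDesplazable) while a BP_CajaInteractiva crate rests on it.
; Box overlap begin and end events, filtered by a cast to the crate, set Apretado and pass it to the wall's SwitchOnOff.
; A timeline plays on press and reverses on release, lerping the Cube's relative Z to sink and raise the plate.
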(event OnComponentBeginOverlap(Box)
  (params (OverlappedComponent :type Primitive%20Component%20Object%20Reference) (OtherActor :type Actor%20Object%20Reference) (OtherComp :type Primitive%20Component%20Object%20Reference) (OtherBodyIndex :type Integer) (bFromSweep :type Boolean) (SweepResult :type Hit%20Result%20Structure%20%28by%20ref%29))
  (Utilities|Casting|CastToBP_CajaInteractiva OtherActor)
  (bind _output_get (Variables|Default|Setapretado true))
  (Default|SwitchOn/Off (Variables|Default|GetParedDesplazable) _output_get)
  (bind _newtrack_0 (Timeline|Timeline_0 Play)
    (:Update
      (Transformation|SetRelativeLocation (Variables|Default|GetCube) (Math|Vector|MakeVector 0.0 0.0 (Math|Float|Lerp 0.0 -1e+01 _newtrack_0)) false false))))

(event OnComponentEndOverlap(Box)
  (params (OverlappedComponent :type Primitive%20Component%20Object%20Reference) (OtherActor :type Actor%20Object%20Reference) (OtherComp :type Primitive%20Component%20Object%20Reference) (OtherBodyIndex :type Integer))
  (Utilities|Casting|CastToBP_CajaInteractiva OtherActor)
  (bind _output_get (Variables|Default|Setapretado false))
  (Default|SwitchOn/Off (Variables|Default|GetParedDesplazable) _output_get)
  (bind _newtrack_0 (Timeline|Timeline_0 Reverse)
    (:Update
      (Transformation|SetRelativeLocation (Variables|Default|GetCube) (Math|Vector|MakeVector 0.0 0.0 (Math|Float|Lerp 0.0 -1e+01 _newtrack_0)) false false))))

(event EventBeginPlay)

(event Collision|EventActorBeginOverlap
  (params (OtherActor :type Actor%20Object%20Reference)))

(event EventTick
  (params (DeltaSeconds :type Float%20%28single-precision%29)))

(fn ConstructionScript)