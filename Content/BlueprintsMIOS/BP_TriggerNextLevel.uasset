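; BP_TriggerNextLevel is a trigger actor that moves the game on to the next level when the player character (BP_Personaje) enters its box.
; On overlap it increments the NumNivel counter in BP_GameInstance and prints the result to the screen.
; It then opens the LevelWin level if that result exceeds one, otherwise Level1, with both level names hard-coded.
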(event OnComponentBeginOverlap(Box)
  (params (OverlappedComponent :type Primitive%20Component%20Object%20Reference) (OtherActor :type Actor%20Object%20Reference) (OtherComp :type Primitive%20Component%20Object%20Reference) (OtherBodyIndex :type Integer) (bFromSweep :type Boolean) (SweepResult :type Hit%20Result%20Structure%20%28by%20ref%29))
  (Utilities|Casting|CastToBP_Personaje OtherActor)
  (bind _asbp_game_instance (Utilities|Casting|CastToBP_GameInstance (Game|GetGameInstance)))
  (bind _result (Math|Integer|IncrementInt (Variables|/Game/GameInstance/BP_GameInstance.BP_GameInstance_C|GetnumNivel _asbp_game_instance))
    (:%20%20
      (Development|PrintString (Utilities|String|ToString(Integer) _result))
      (if (> _result 1)
        (Game|OpenLevel(byName) "LevelWin")
        (else
          (Game|OpenLevel(byName) "Level1"))))))

(event EventBeginPlay)

(event Collision|EventActorBeginOverlap
  (params (OtherActor :type Actor%20Object%20Reference)))

(event EventTick
  (params (DeltaSeconds :type Float%20%28single-precision%29)))

(fn ConstructionScript)